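; BP_PlayerController is a physics-driven rolling ball control Blueprint that turns player input into forces on its Sphere component.
; The MoveForward and MoveRight axes apply torque around the world Y and X axes, scaled by RollTorque and negated, so movement comes from rolling.
; A left mouse press applies a single small constant-falloff radial force to the same sphere.
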(event Input|AxisEvents|InputAxisMoveForward
  (params (AxisValue :type Float%20%28single-precision%29))
  ;[1 0 0.01667 0.686] Move Forward & Backward
  (Class|PrimitiveComponent|AddTorqueinRadians (Variables|Default|GetSphere) (Math|Vector|MakeVector 0.0 (* (Variables|Default|GetRollTorque) AxisValue -1.0) 0.0) "None" false))

(event Input|AxisEvents|InputAxisMoveRight
  (params (AxisValue :type Float%20%28single-precision%29))
  ;[1 0 0.02469 0.686] Move Left & Right
  (Class|PrimitiveComponent|AddTorqueinRadians (Variables|Default|GetSphere) (Math|Vector|MakeVector (* (Variables|Default|GetRollTorque) AxisValue -1.0) 0.0 0.0) "None" false))

(event Input|MouseEvents|LeftMouseButton
  (params (Key :type Key%20Structure :default "None"))
  (:Pressed
    (Physics|AddRadialForce (Variables|Default|GetSphere) "0, 0, 0" 1.0 4.0 "RIF_Constant" false)))

(fn ConstructionScript)